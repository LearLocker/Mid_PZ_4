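; AppleBP is an apple pickup that heals the player and is consumed on contact.
; When its static mesh is hit by a ThirdPersonCharacter, it adds a fixed amount to CurrentHealth, or sets it to Health if already at or above that value.
; The addition is not clamped, so health can overshoot Health.
; In either case the apple destroys itself and decrements the character's FoodCounter.
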(event `self.StaticMesh.OnComponentHit`
  (params (HitComponent :type "PrimitiveComponent Object Reference") (OtherActor :type "Actor Object Reference") (OtherComp :type "PrimitiveComponent Object Reference") (NormalImpulse :type "Vector Structure") (Hit :type "HitResult Structure (by ref)"))
  (bind _asthird_person_character (cast `/Game/ThirdPersonBP/Blueprints/ThirdPersonCharacter` OtherActor))
  (bind _current_health (`/Game/ThirdPersonBP/Blueprints/ThirdPersonCharacter.Current Health` _asthird_person_character))
  (bind _health (`/Game/ThirdPersonBP/Blueprints/ThirdPersonCharacter.Health` _asthird_person_character))
  (if (>= _current_health _health)
    (set `/Game/ThirdPersonBP/Blueprints/ThirdPersonCharacter.Current Health` _health _asthird_person_character)
    (else
      (set `/Game/ThirdPersonBP/Blueprints/ThirdPersonCharacter.Current Health` (+ _current_health 500.0) _asthird_person_character)))
  (`self.K2_DestroyActor`)
  (bind _result (`/Engine/EditorBlueprintResources/StandardMacros.DecrementFloat` (`/Game/ThirdPersonBP/Blueprints/ThirdPersonCharacter.FoodCounter` _asthird_person_character))
    (:`  `
      (set `/Game/ThirdPersonBP/Blueprints/ThirdPersonCharacter.FoodCounter` _result _asthird_person_character))))

(fn `UserConstructionScript`)